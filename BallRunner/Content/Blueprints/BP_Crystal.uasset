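; BP_Crystal is a crystal actor that is drawn into the player and vanishes when the player pawn overlaps it.
; The overlap caches the crystal's location and scale, then plays a timeline with separate move and scale curves.
; Each update lerps it toward the pawn's current location and shrinks it toward zero scale, and the actor is destroyed when the timeline finishes.
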(event `self.ReceiveActorBeginOverlap`
  (params (OtherActor :type "Actor Object Reference"))
  (if (== OtherActor (`GameplayStatics.GetPlayerPawn` 0))
    (`self.SetActualCrystalValues`)
    (bind (_direction _smooth_lerp_alpha _scale_lerp_alpha) (`Timeline|Smooth Lerp Alpha`)
      (:`Update`
        (`self.SetLerpMoveCrystal` _smooth_lerp_alpha)
        (`self.SetLerpScaleCrystal` _scale_lerp_alpha))
      (:`Finished`
        (`self.K2_DestroyActor`)))))

(fn `SetActualCrystalValues`
  (set `self.CrystalActualLoc` (`self.K2_GetActorLocation`))
  (set `self.CrystalActualScale` (`self.GetActorScale3D`)))

(fn `SetLerpMoveCrystal`
  (params (Alpha :type "Float (double-precision)"))
  (`self.K2_SetActorLocation` (`KismetMathLibrary.VLerp` (`self.CrystalActualLoc`) (`self.K2_GetActorLocation` (`GameplayStatics.GetPlayerPawn` 0)) Alpha)))

(fn `SetLerpScaleCrystal`
  (params (Alpha :type "Float (double-precision)"))
  (`self.SetActorScale3D` (`KismetMathLibrary.VLerp` (`self.CrystalActualScale`) (0.0 0.0 0.0) Alpha)))

(fn `UserConstructionScript`)